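; Blueprint that triggers the Dancheong petal and cherry blossom Niagara effects placed in the level.
; The DancheongPetals_VFX event activates the first Niagara actor in the level, while Cherry_Blossom_VFX uses ResultIndex to pick one of six others.
; Each branch finds its target by a hard-coded, non-sequential index into GetAllActorsOfClass, so the mapping depends on the order of that returned array.
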(event Custom|DancheongPetals_VFX
  (bind _outactors (Actor|GetAllActorsOfClass "/Script/Niagara.NiagaraActor"))
  (bind _as나이아가라_액터 (Utilities|Casting|CastToNiagaraActor (Utilities|Array|Get(acopy) _outactors)))
  (Components|Activation|Activate (Variables|/Script/Niagara.NiagaraActor|GetNiagaraComponent _as나이아가라_액터) false))

(event Custom|Cherry_Blossom_VFX
  (params (ResultIndex :type Integer))
  (switch int ResultIndex
    (:1
      (bind _outactors (Actor|GetAllActorsOfClass "/Script/Niagara.NiagaraActor"))
      (bind _as나이아가라_액터 (Utilities|Casting|CastToNiagaraActor (Utilities|Array|Get(acopy) _outactors 4)))
      (Components|Activation|Activate (Variables|/Script/Niagara.NiagaraActor|GetNiagaraComponent _as나이아가라_액터) false))
    (:2
      (bind _outactors_2 (Actor|GetAllActorsOfClass "/Script/Niagara.NiagaraActor"))
      (bind _as나이아가라_액터_2 (Utilities|Casting|CastToNiagaraActor (Utilities|Array|Get(acopy) _outactors_2 2)))
      (Components|Activation|Activate (Variables|/Script/Niagara.NiagaraActor|GetNiagaraComponent _as나이아가라_액터_2) false))
    (:3
      (bind _outactors_3 (Actor|GetAllActorsOfClass "/Script/Niagara.NiagaraActor"))
      (bind _as나이아가라_액터_3 (Utilities|Casting|CastToNiagaraActor (Utilities|Array|Get(acopy) _outactors_3 6)))
      (Components|Activation|Activate (Variables|/Script/Niagara.NiagaraActor|GetNiagaraComponent _as나이아가라_액터_3) false))
    (:4
      (bind _outactors_4 (Actor|GetAllActorsOfClass "/Script/Niagara.NiagaraActor"))
      (bind _as나이아가라_액터_4 (Utilities|Casting|CastToNiagaraActor (Utilities|Array|Get(acopy) _outactors_4 3)))
      (Components|Activation|Activate (Variables|/Script/Niagara.NiagaraActor|GetNiagaraComponent _as나이아가라_액터_4) false))
    (:5
      (bind _outactors_5 (Actor|GetAllActorsOfClass "/Script/Niagara.NiagaraActor"))
      (bind _as나이아가라_액터_5 (Utilities|Casting|CastToNiagaraActor (Utilities|Array|Get(acopy) _outactors_5 5)))
      (Components|Activation|Activate (Variables|/Script/Niagara.NiagaraActor|GetNiagaraComponent _as나이아가라_액터_5) false))
    (:6
      (bind _outactors_6 (Actor|GetAllActorsOfClass "/Script/Niagara.NiagaraActor"))
      (bind _as나이아가라_액터_6 (Utilities|Casting|CastToNiagaraActor (Utilities|Array|Get(acopy) _outactors_6 1)))
      (Components|Activation|Activate (Variables|/Script/Niagara.NiagaraActor|GetNiagaraComponent _as나이아가라_액터_6) false))))

(fn ConstructionScript)