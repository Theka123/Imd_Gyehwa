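; BP_SkyChanger animates the level's BP_GoodSky, changing its time of day and overlay color on request.
; ChangeSkyTime plays a timeline that feeds TimeOfDayForCustomMode into the sky's TimelineAnimation with VFX on.
; ChangeSkyColor switches on ResultIndex to one of six tint presets, each with its own timeline.
; Each timeline lerps GlobalOverlayColor from its current value toward the preset and applies it through TimelineColor.
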(event Custom|ChangeSkyTime
  (bind _outactors (Actor|GetAllActorsOfClass "/Game/GoodSky/Blueprint/BP_GoodSky.BP_GoodSky_C"))
  (bind _asbp_good_sky (Utilities|Casting|CastToBP_GoodSky (Utilities|Array|Get(acopy) _outactors)))
  (bind _timevalue (Timeline|타임라인 Play)
    (:Update
      (bind _output_get (Variables|/Game/GoodSky/Blueprint/BP_GoodSky.BP_GoodSky_C|Set└%20Time%20of%20Day%20%28%20For%20Custom%20Mode%20%29 _asbp_good_sky _timevalue))
      (Default|TimelineAnimation _asbp_good_sky _output_get true))))

(event Custom|ChangeSkyColor
  (params (ResultIndex :type Integer))
  (switch int ResultIndex
    (:1
      ;[0.15 0.15 0.15 0.5] 빨강
      (bind _outactors (Actor|GetAllActorsOfClass "/Game/GoodSky/Blueprint/BP_GoodSky.BP_GoodSky_C"))
      (bind _alpha (Timeline|타임라인_0 Play)
        (:Update
          (bind _output_get (Variables|/Game/GoodSky/Blueprint/BP_GoodSky.BP_GoodSky_C|SetGlobal%20Overlay%20Color (Utilities|Array|Get(acopy) _outactors) (Math|Color|Lerp(LinearColor) (Variables|/Game/GoodSky/Blueprint/BP_GoodSky.BP_GoodSky_C|GetGlobal%20Overlay%20Color (Utilities|Array|Get(acopy) _outactors)) (Utilities|Struct|MakeLinearColor 0.78125 0.549316 0.549316 1.0) _alpha)))
          (Default|TimelineColor (Utilities|Array|Get(acopy) _outactors) _output_get))))
    (:2
      ;[0.15 0.15 0.15 0.5] 노랑
      (bind _outactors_2 (Actor|GetAllActorsOfClass "/Game/GoodSky/Blueprint/BP_GoodSky.BP_GoodSky_C"))
      (bind _alpha_2 (Timeline|타임라인_2 Play)
        (:Update
          (bind _output_get_2 (Variables|/Game/GoodSky/Blueprint/BP_GoodSky.BP_GoodSky_C|SetGlobal%20Overlay%20Color (Utilities|Array|Get(acopy) _outactors_2) (Math|Color|Lerp(LinearColor) (Variables|/Game/GoodSky/Blueprint/BP_GoodSky.BP_GoodSky_C|GetGlobal%20Overlay%20Color (Utilities|Array|Get(acopy) _outactors_2)) (Utilities|Struct|MakeLinearColor 0.84375 0.795557 0.637207 1.0) _alpha_2)))
          (Default|TimelineColor (Utilities|Array|Get(acopy) _outactors_2) _output_get_2))))
    (:3
      ;[0.15 0.15 0.15 0.5] 초록
      (bind _outactors_3 (Actor|GetAllActorsOfClass "/Game/GoodSky/Blueprint/BP_GoodSky.BP_GoodSky_C"))
      (bind _alpha_3 (Timeline|타임라인_3 Play)
        (:Update
          (bind _output_get_3 (Variables|/Game/GoodSky/Blueprint/BP_GoodSky.BP_GoodSky_C|SetGlobal%20Overlay%20Color (Utilities|Array|Get(acopy) _outactors_3) (Math|Color|Lerp(LinearColor) (Variables|/Game/GoodSky/Blueprint/BP_GoodSky.BP_GoodSky_C|GetGlobal%20Overlay%20Color (Utilities|Array|Get(acopy) _outactors_3)) (Utilities|Struct|MakeLinearColor 0.342936 0.765625 0.39225 1.0) _alpha_3)))
          (Default|TimelineColor (Utilities|Array|Get(acopy) _outactors_3) _output_get_3))))
    (:4
      ;[0.15 0.15 0.15 0.5] 파랑
      (bind _outactors_4 (Actor|GetAllActorsOfClass "/Game/GoodSky/Blueprint/BP_GoodSky.BP_GoodSky_C"))
      (bind _alpha_4 (Timeline|타임라인_1 Play)
        (:Update
          (bind _output_get_4 (Variables|/Game/GoodSky/Blueprint/BP_GoodSky.BP_GoodSky_C|SetGlobal%20Overlay%20Color (Utilities|Array|Get(acopy) _outactors_4) (Math|Color|Lerp(LinearColor) (Variables|/Game/GoodSky/Blueprint/BP_GoodSky.BP_GoodSky_C|GetGlobal%20Overlay%20Color (Utilities|Array|Get(acopy) _outactors_4)) (Utilities|Struct|MakeLinearColor 0.341064 0.434163 0.515625 1.0) _alpha_4)))
          (Default|TimelineColor (Utilities|Array|Get(acopy) _outactors_4) _output_get_4))))
    (:5
      ;[0.15 0.15 0.15 0.5] 흰색
      (bind _outactors_5 (Actor|GetAllActorsOfClass "/Game/GoodSky/Blueprint/BP_GoodSky.BP_GoodSky_C"))
      (bind _alpha_5 (Timeline|타임라인_4 Play)
        (:Update
          (bind _output_get_5 (Variables|/Game/GoodSky/Blueprint/BP_GoodSky.BP_GoodSky_C|SetGlobal%20Overlay%20Color (Utilities|Array|Get(acopy) _outactors_5) (Math|Color|Lerp(LinearColor) (Variables|/Game/GoodSky/Blueprint/BP_GoodSky.BP_GoodSky_C|GetGlobal%20Overlay%20Color (Utilities|Array|Get(acopy) _outactors_5)) (Utilities|Struct|MakeLinearColor 0.734375 0.694405 0.516357 1.0) _alpha_5)))
          (Default|TimelineColor (Utilities|Array|Get(acopy) _outactors_5) _output_get_5))))
    (:6
      ;[0.15 0.15 0.15 0.5] 검정
      (bind _outactors_6 (Actor|GetAllActorsOfClass "/Game/GoodSky/Blueprint/BP_GoodSky.BP_GoodSky_C"))
      (bind _alpha_6 (Timeline|타임라인_5 Play)
        (:Update
          (bind _output_get_6 (Variables|/Game/GoodSky/Blueprint/BP_GoodSky.BP_GoodSky_C|SetGlobal%20Overlay%20Color (Utilities|Array|Get(acopy) _outactors_6) (Math|Color|Lerp(LinearColor) (Variables|/Game/GoodSky/Blueprint/BP_GoodSky.BP_GoodSky_C|GetGlobal%20Overlay%20Color (Utilities|Array|Get(acopy) _outactors_6)) (Utilities|Struct|MakeLinearColor 0.288818 0.304846 0.609375 1.0) _alpha_6)))
          (Default|TimelineColor (Utilities|Array|Get(acopy) _outactors_6) _output_get_6))))))

(fn ConstructionScript)