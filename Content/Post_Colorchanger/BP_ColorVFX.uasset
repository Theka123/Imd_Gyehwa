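; BP_ColorVFX is an actor that changes the sky and post-process color look at runtime.
; Its VFX_sky/post event triggers sky color and time changes on BP_SkyChanger, applies preset 1, and disables the first PostProcessVolume found.
; ApplyVisualPreset copies settings from a DT_VisualPresets row into the third volume found, then uses a timeline to lerp its BlendWeight to full.
; Volumes are picked by GetAllActorsOfClass index, so targeting depends on actor order.
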(event Custom|ApplyVisualPreset
  (params (ResultID :type Integer))
  ;[0.15 0.15 0.15 0.5] 포스트프로세스 컬러 블랜드 & 변경
  (bind _returnvalue (Utilities|GetDataTableRow "/Game/Post_Colorchanger/DT_VisualPresets.DT_VisualPresets" (Utilities|String|StringToName (Utilities|String|ToString(Integer) ResultID)))
    (:then
      (bind _outactors (Actor|GetAllActorsOfClass "/Script/Engine.PostProcessVolume"))
      (bind _as포스트_프로세스_볼륨 (Utilities|Casting|CastToPostProcessVolume (Utilities|Array|Get(acopy) _outactors 2)))
      (Variables|Default|SetStartBlendWeight (Variables|/Script/Engine.PostProcessVolume|GetBlendWeight _as포스트_프로세스_볼륨))
      (Variables|Default|SetTargetBlendWeight 1.0)
      (Variables|/Script/Engine.PostProcessVolume|SetSettings _as포스트_프로세스_볼륨 (Utilities|Struct|BreakSTR_VisualPresetRow _returnvalue))
      (bind _alpha (Timeline|Timeline PlayFromStart)
        (:Update
          (Variables|/Script/Engine.PostProcessVolume|SetBlendWeight _as포스트_프로세스_볼륨 (Math|Float|Lerp (Variables|Default|GetStartBlendWeight) (Variables|Default|GetTargetBlendWeight) _alpha)))))))

(event Custom|VFX_sky/post
  (bind _outactors (Actor|GetAllActorsOfClass "/Game/Post_Colorchanger/BP_SkyChanger.BP_SkyChanger_C"))
  (bind _asbp_sky_changer (Utilities|Casting|CastToBP_SkyChanger (Utilities|Array|Get(acopy) _outactors)))
  (Default|ChangeSkyColor _asbp_sky_changer)
  ;[0.15 0.15 0.15 0.5] 시간변경 / 기존 정자 내 포스트프로세싱 꺼짐 -> 셋팅 포스트프로세스 호출
  (bind _outactors_2 (Actor|GetAllActorsOfClass "/Game/Post_Colorchanger/BP_SkyChanger.BP_SkyChanger_C"))
  (bind _asbp_sky_changer_2 (Utilities|Casting|CastToBP_SkyChanger (Utilities|Array|Get(acopy) _outactors_2)))
  (Default|ChangeSkyTime _asbp_sky_changer_2)
  (CallFunction|ApplyVisualPreset 1)
  (bind _outactors_3 (Actor|GetAllActorsOfClass "/Script/Engine.PostProcessVolume"))
  (bind _as포스트_프로세스_볼륨 (Utilities|Casting|CastToPostProcessVolume (Utilities|Array|Get(acopy) _outactors_3)))
  (Timeline|Timeline_0 Play
    (:Update
      (Variables|/Script/Engine.PostProcessVolume|SetbEnabled _as포스트_프로세스_볼륨 false))))

(event EventBeginPlay)

(fn ConstructionScript)