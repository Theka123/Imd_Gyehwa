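; Background music player actor that switches between main, tutorial and VFX music tracks.
; It starts the main track on BeginPlay and exposes events to play each of the three tracks.
; Each event stops or fades out the other two audio components before starting its own.
; The VFX switch overlaps a fade-out of the main track with a delayed fade-in of the VFX track.
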(event Custom|Play_VFX_BGM
  (Audio|Components|Audio|Stop (Variables|Default|GetAudio_Tutorial))
  (Audio|Components|Audio|FadeOut (Variables|Default|GetAudio_Main) 2.0 0.0 "Linear" :!class /Script/Engine.AudioComponent)
  (Utilities|FlowControl|Delay 1.5)
  (Audio|Components|Audio|FadeIn (Variables|Default|GetAudio_VFX) 2.0 1.0 0.0 "Linear" :!class /Script/Engine.AudioComponent))

(event Custom|Play_Tutorial_BGM
  (Audio|Components|Audio|Stop (Variables|Default|GetAudio_Main))
  (Audio|Components|Audio|Stop (Variables|Default|GetAudio_VFX))
  (Audio|Components|Audio|Play (Variables|Default|GetAudio_Tutorial) 0.0))

(event Custom|Play_Main_BGM
  (Audio|Components|Audio|FadeOut (Variables|Default|GetAudio_Tutorial) 0.0 0.0 "Linear" :!class /Script/Engine.AudioComponent)
  (Audio|Components|Audio|Stop (Variables|Default|GetAudio_VFX))
  (Audio|Components|Audio|FadeIn (Variables|Default|GetAudio_Main) 0.0 1.0 0.0 "Linear" :!class /Script/Engine.AudioComponent))

(event EventBeginPlay
  (Audio|Components|Audio|FadeIn (Variables|Default|GetAudio_Main) 0.0 1.0 0.0 "Linear" :!class /Script/Engine.AudioComponent))

(fn ConstructionScript)