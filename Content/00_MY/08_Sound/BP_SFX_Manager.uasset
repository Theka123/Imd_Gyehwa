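; BP_SFX_Manager is a sound effects manager actor for a coloring game's interface and feedback sounds.
; It exposes one event each for UI click, palette selection, coloring, dissolve, coloring completion and transition.
; Each event plays its sound as non-spatialized 2D audio, with no further logic.
; The coloring event uses the second version of its sound, leaving the original SFXColoring unused.
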(event Custom|Play_SFX_Complete_Coloring
  (Audio|PlaySound2D (Variables|Default|GetSFX_Complete_Coloring) 1.0 1.0 0.0 0 0))

(event Custom|Play_SFX_UI_Click
  (Audio|PlaySound2D (Variables|Default|GetSFX_UI_Click) 1.0 1.0 0.0 0 0))

(event Custom|Play_SFX_Dissolve
  (Audio|PlaySound2D (Variables|Default|GetSFX_Dissolve) 1.0 1.0 0.0 0 0))

(event Custom|Play_SFX_Palette_Select
  (Audio|PlaySound2D (Variables|Default|GetSFX_Palette_Select) 1.0 1.0 0.0 0 0))

(event Custom|Play__SFX_Transition
  (Audio|PlaySound2D (Variables|Default|GetSFX_Transition) 1.0 1.0 0.0 0 0))

(event Custom|Play_SFX_Coloring
  (Audio|PlaySound2D (Variables|Default|GetSFX_Coloring_ver2) 1.0 1.0 0.0 0 0))

(fn ConstructionScript)