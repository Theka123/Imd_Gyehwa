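; BP_SFX_Naration is a sound Blueprint that plays narration clips through its AudioNaration audio component.
; Its sfx_nara_play event stops current playback, takes the first BPA_NARATION actor in the level and calls IndexSync on it.
; It then uses that actor's BPAINDEX to pick a clip from the NarationSound array and plays it from the start.
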(event Custom|sfx_nara_play
  (Audio|Components|Audio|Stop (Variables|Default|GetAudio_naration))
  (bind _outactors (Actor|GetAllActorsOfClass "/Game/00_MY/05_UI/BPA_NARATION.BPA_NARATION_C"))
  (bind _asbpa_naration (Utilities|Casting|CastToBPA_NARATION (Utilities|Array|Get(acopy) _outactors)))
  (Default|IndexSync _asbpa_naration)
  (Audio|Components|Audio|SetSound (Variables|Default|GetAudio_naration) (Utilities|Array|Get(acopy) (Variables|Default|GetNaration_Sound) (Variables|/Game/00_MY/05_UI/BPA_NARATION.BPA_NARATION_C|GetBPA_INDEX _asbpa_naration)))
  (Audio|Components|Audio|Play (Variables|Default|GetAudio_naration) 0.0))

(fn ConstructionScript)