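; BP_Dancheong is a colouring Blueprint for dancheong pieces, swapping mesh materials when a tagged component overlaps one of five trigger boxes.
; Each box's begin-overlap checks for a colour tag, then sets slot 0 on a dancheong mesh to a fixed material.
; Boxes 1–3 drive their same-numbered meshes, while 4 and 5 both drive SMDancheong4.
; Box 4 applies red on the "Yellow" tag, and nothing reverts the materials.
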(event OnComponentBeginOverlap(Dan1_Box)
  (params (OverlappedComponent :type Primitive%20Component%20Object%20Reference) (OtherActor :type Actor%20Object%20Reference) (OtherComp :type Primitive%20Component%20Object%20Reference) (OtherBodyIndex :type Integer) (bFromSweep :type Boolean) (SweepResult :type Hit%20Result%20Structure%20%28by%20ref%29))
  (if (Components|ComponentHasTag OtherComp "White")
    (Rendering|Material|SetMaterial (Variables|Default|GetSM_Dancheong1) 0 "/Game/00_MY/03_Materials/02_Dancheong/M_DanBasic1.M_DanBasic1")))

(event OnComponentBeginOverlap(Dan2_Box)
  (params (OverlappedComponent :type Primitive%20Component%20Object%20Reference) (OtherActor :type Actor%20Object%20Reference) (OtherComp :type Primitive%20Component%20Object%20Reference) (OtherBodyIndex :type Integer) (bFromSweep :type Boolean) (SweepResult :type Hit%20Result%20Structure%20%28by%20ref%29))
  (if (Components|ComponentHasTag OtherComp "Blue")
    (Rendering|Material|SetMaterial (Variables|Default|GetSM_Dancheong2) 0 "/Game/00_MY/03_Materials/02_Dancheong/M_DanBlue.M_DanBlue")))

(event OnComponentBeginOverlap(Dan3_Box)
  (params (OverlappedComponent :type Primitive%20Component%20Object%20Reference) (OtherActor :type Actor%20Object%20Reference) (OtherComp :type Primitive%20Component%20Object%20Reference) (OtherBodyIndex :type Integer) (bFromSweep :type Boolean) (SweepResult :type Hit%20Result%20Structure%20%28by%20ref%29))
  (if (Components|ComponentHasTag OtherComp "Yellow")
    (Rendering|Material|SetMaterial (Variables|Default|GetSM_Dancheong3) 0 "/Game/00_MY/03_Materials/02_Dancheong/M_DanYellow.M_DanYellow")))

(event OnComponentBeginOverlap(Dan4_Box)
  (params (OverlappedComponent :type Primitive%20Component%20Object%20Reference) (OtherActor :type Actor%20Object%20Reference) (OtherComp :type Primitive%20Component%20Object%20Reference) (OtherBodyIndex :type Integer) (bFromSweep :type Boolean) (SweepResult :type Hit%20Result%20Structure%20%28by%20ref%29))
  (if (Components|ComponentHasTag OtherComp "Yellow")
    (Rendering|Material|SetMaterial (Variables|Default|GetSM_Dancheong4) 0 "/Game/00_MY/03_Materials/02_Dancheong/M_DanRed.M_DanRed")))

(event OnComponentBeginOverlap(Dan5_Box)
  (params (OverlappedComponent :type Primitive%20Component%20Object%20Reference) (OtherActor :type Actor%20Object%20Reference) (OtherComp :type Primitive%20Component%20Object%20Reference) (OtherBodyIndex :type Integer) (bFromSweep :type Boolean) (SweepResult :type Hit%20Result%20Structure%20%28by%20ref%29))
  (if (Components|ComponentHasTag OtherComp "Green")
    (Rendering|Material|SetMaterial (Variables|Default|GetSM_Dancheong4) 0 "/Game/00_MY/03_Materials/02_Dancheong/M_DanGreen.M_DanGreen")))

(event EventBeginPlay)

(event Collision|EventActorBeginOverlap
  (params (OtherActor :type Actor%20Object%20Reference)))

(event EventTick
  (params (DeltaSeconds :type Float%20%28single-precision%29)))

(fn ConstructionScript)