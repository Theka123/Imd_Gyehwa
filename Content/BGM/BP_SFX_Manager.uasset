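; BP_SFX_Manager is a sound effect manager Blueprint for the game's UI and coloring interactions.
; It exposes custom events for UI click, palette select, coloring and dissolve effects.
; Each event plays its own sound variable as non-spatialized 2D audio, with no other logic or state handling.
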(event Custom|Play_Dissolve_SFX
  (Audio|PlaySound2D (Variables|Default|GetSFX_Dissolve) 1.0 1.0 0.0 0 0))

(event Custom|Play_UI_Click_SFX
  (Audio|PlaySound2D (Variables|Default|GetSFX_UI_Click) 1.0 1.0 0.0 0 0))

(event Custom|Play_Palette_Select_SFX
  (Audio|PlaySound2D (Variables|Default|GetSFX_Palette_Select) 1.0 1.0 0.0 0 0))

(event Custom|Play_Coloring_SFX
  (Audio|PlaySound2D (Variables|Default|GetSFX_Coloring) 1.0 1.0 0.0 0 0))

(fn ConstructionScript)